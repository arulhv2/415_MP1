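; BP_Projectile is a player shot that flies forward, destroys enemies and awards score.
; Each Tick it sweeps along world X at a base speed plus the player's ForwardSpeed, and destroys itself after a fixed count of ticks rather than elapsed time.
; Any sphere overlap destroys it; hitting a BP_Enemy also destroys that enemy, then adds to the player's Score and refreshes the WBScore widget.
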(event OnComponentBeginOverlap(Sphere)
  (params (OverlappedComponent :type Primitive%20Component%20Object%20Reference) (OtherActor :type Actor%20Object%20Reference) (OtherComp :type Primitive%20Component%20Object%20Reference) (OtherBodyIndex :type Integer) (bFromSweep :type Boolean) (SweepResult :type Hit%20Result%20Structure%20%28by%20ref%29))
  (bind _asbp_enemy (Utilities|Casting|CastToBP_Enemy OtherActor)
    (:then
      (Actor|DestroyActor _asbp_enemy)
      (Actor|DestroyActor)
      (bind _asbp_player (Utilities|Casting|CastToBP_Player (Game|Player|GetPlayerPawn 0)))
      (bind _output_get (Variables|/Game/InfiniteMatrix/Blueprints/BP_Player.BP_Player_C|SetScore _asbp_player (+ (Variables|/Game/InfiniteMatrix/Blueprints/BP_Player.BP_Player_C|GetScore _asbp_player) 1e+01)))
      (Default|UpdateScore (Variables|/Game/InfiniteMatrix/Blueprints/BP_Player.BP_Player_C|GetWBScore _asbp_player) _output_get))
    (:CastFailed
      (Actor|DestroyActor))))

(event EventTick
  (params (DeltaSeconds :type Float%20%28single-precision%29))
  (bind _asbp_player (Utilities|Casting|CastToBP_Player (Game|Player|GetPlayerPawn 0)))
  (Transformation|AddActorWorldOffset (Math|Vector|MakeVector (* DeltaSeconds (+ 5e+02 (Variables|/Game/InfiniteMatrix/Blueprints/BP_Player.BP_Player_C|GetForwardSpeed _asbp_player))) 0.0 0.0) true)
  (bind _output_get (Variables|Default|SetTime (+ (Variables|Default|GetTime) 1)))
  (if (== _output_get 200)
    (Actor|DestroyActor)))

(fn ConstructionScript)